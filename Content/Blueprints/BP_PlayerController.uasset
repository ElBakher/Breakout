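; Player controller for a paddle-and-brick game that passes player input to the paddle pawn.
; On BeginPlay it sets game-only input and caches paddle and game mode references through message calls.
; The movement axis and release-ball action drive the paddle.
; A T-key cheat destroys all bricks, clears the grid's spawned list, flags the game mode as waiting for a new level, and calls DestroyActor on itself.
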(event `self.ReceiveBeginPlay`
  (`|ExecutionSequence`
    (:`then_0`
      (`WidgetBlueprintLibrary.SetInputMode_GameOnly` self))
    (:`then_1`
      (bind _paddleref (message `/Game/Blueprints/Interfaces/BI_GetPaddle.GetPaddleRef` (`GameplayStatics.GetPlayerPawn` 0)))
      (set `self.BP_Paddle` _paddleref)
      (bind _gamemoderef (message `/Game/Blueprints/Interfaces/BI_GetGameMode.GetGameModeRef` (`GameplayStatics.GetGameMode`)))
      (set `self.BP_GameMode` _gamemoderef))))

(event `InputAxis|PaddleMovement`
  (params (AxisValue :type "Float (single-precision)"))
  (`/Game/Blueprints/BP_Paddle.ProcessMovementInput` (`self.BP_Paddle`) AxisValue))

(event `InputAction|ReleaseBall`
  (params (Key :type "Key Structure"))
  (:`Pressed`
    (`/Game/Blueprints/BP_Paddle.ReleaseBall` (`self.BP_Paddle`))))

(event `Key|T`
  (params (Key :type "Key Structure"))
  (:`Pressed`
    (`self.CheatThroughLevel`)))

(fn `CheatThroughLevel`
  (locals (grid :type "/Game/Blueprints/Actors/BP_GridForBricks Object Reference"))
  (bind _outactors (`GameplayStatics.GetAllActorsOfClass` "/Game/Blueprints/Actors/Bricks/BP_BrickBase.BP_BrickBase_C"))
  (for _array_element _outactors
    (`self.K2_DestroyActor` _array_element)
    (bind _outactors_2 (`GameplayStatics.GetAllActorsOfClass` "/Game/Blueprints/Actors/BP_GridForBricks.BP_GridForBricks_C"))
    (bind _output_get (set `local.grid` (`|GetArrayItem` _outactors_2)))
    (`KismetArrayLibrary.Array_Clear` (`/Game/Blueprints/Actors/BP_GridForBricks.spawnedBricks` _output_get))
    (set `/Game/Blueprints/BP_GameMode.waitingForNewLevel` true (`self.BP_GameMode`))
    (`self.K2_DestroyActor`)))

(fn `GetPlayerController`
  (returns (controllerRef :type "/Game/Blueprints/BP_PlayerController Object Reference"))
  (return self))

(fn `UserConstructionScript`)