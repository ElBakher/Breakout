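; Player paddle for a ball-bouncing game that sweeps along Y from axis input, spawns an attached ball and releases it.
; On hits from BI_GetBall actors, it plays a sound and adjusts the game mode's ball reflection by impact offset, normalised to mesh half-width and scaled by sensitivity.
; The construction script caches that half-width from mesh bounds.
; Spread shot is a stub that only prints a debug string.
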(event `self.ReceiveBeginPlay`
  (bind _gamemoderef (message `/Game/Blueprints/Interfaces/BI_GetGameMode.GetGameModeRef` (`GameplayStatics.GetGameMode`)))
  (set `self.BP_GameMode` _gamemoderef))

(event `self.PaddleMesh.OnComponentHit`
  (params (HitComponent :type "PrimitiveComponent Object Reference") (OtherActor :type "Actor Object Reference") (OtherComp :type "PrimitiveComponent Object Reference") (NormalImpulse :type "Vector Structure") (Hit :type "HitResult Structure (by ref)"))
  (bind (_bblockinghit _binitialoverlap _time _distance _location _impactpoint) (`GameplayStatics.BreakHitResult` Hit))
  (`/Game/Blueprints/MacroLibrary.DoesImplementInterface` OtherActor "/Game/Blueprints/Interfaces/BI_GetBall.BI_GetBall_C"
    (:`True`
      (`GameplayStatics.PlaySoundAtLocation` (`self.ballHitSound`) _location (struct) 1.0 1.0 0.0 null null null)
      (`/Game/Blueprints/Actors/BP_Ball.AdjustReflectedVelocity` (`/Game/Blueprints/BP_GameMode.BP_Ball` (`self.BP_GameMode`)) (* (* (`KismetMathLibrary.MakeVector` 0.0 1.0) (`self.GetDirScalingCoefficient` _impactpoint)) (`self.reflectionDirSensitivityCoefficient`))))))

(fn `ActivateSpreadShot`
  (`KismetSystemLibrary.PrintString` "sebrals spread shot"))

(fn `GetDirScalingCoefficient`
  (params (InVec :type "Vector Structure"))
  (returns (ReturnValue :type "Float (double-precision)"))
  (bind (_returnvalue_x _returnvalue_y) (`KismetMathLibrary.BreakVector` (`self.K2_GetActorLocation`)))
  (return (/ (- (.y InVec) _returnvalue_y) (`self.meshHalfSizeY`))))

(fn `GetPaddleRef`
  (returns (paddleRef :type "/Game/Blueprints/BP_Paddle Object Reference"))
  (return self))

(fn `ProcessMovementInput`
  (params (axisValue :type "Float (double-precision)"))
  (`self.K2_AddActorLocalOffset` (`KismetMathLibrary.MakeVector` 0.0 (* axisValue (`GameplayStatics.GetWorldDeltaSeconds`) (`self.movementSpeed`))) true))

(fn `ReleaseBall`
  (if (not (`/Game/Blueprints/Actors/BP_Ball.isMoving` (`/Game/Blueprints/BP_GameMode.BP_Ball` (`self.BP_GameMode`))))
    (`self.K2_DetachFromActor` (`/Game/Blueprints/BP_GameMode.BP_Ball` (`self.BP_GameMode`)) "KeepWorld" "KeepWorld" "KeepWorld")
    (`/Game/Blueprints/Actors/BP_Ball.StartMoving` (`/Game/Blueprints/BP_GameMode.BP_Ball` (`self.BP_GameMode`)))))

(fn `SpawnNewBall`
  (returns (ballReference :type "/Game/Blueprints/Actors/BP_Ball Object Reference"))
  (locals (SpawnedBall :type "/Game/Blueprints/Actors/BP_Ball Object Reference"))
  (bind _returnvalue (`|SpawnActorFromClass` "/Game/Blueprints/Actors/BP_Ball.BP_Ball_C" (`KismetMathLibrary.MakeTransform` (0.0 0.0 0.0)) "AlwaysSpawn" "OverrideRootScale" null null))
  (bind _output_get (set `local.SpawnedBall` _returnvalue))
  (`self.K2_AttachToComponent` _output_get (`self.BallSpawnPoint`) "None" "SnapToTarget" "SnapToTarget" "SnapToTarget" true)
  (return (`local.SpawnedBall`)))

(fn `UserConstructionScript`
  (set `self.meshHalfSizeY` (.y (`.BoxExtent` (`KismetSystemLibrary.GetComponentBounds` (`self.PaddleMesh`))))))