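; Menu game mode Blueprint that sets up the paddle-and-ball scene and applies saved settings on start.
; On BeginPlay it fetches the paddle from the player pawn through a reference message and has it spawn a ball, caching both.
; It then gets the game instance the same way, loads saved data and applies each temporary audio setting.
; GetGameModeRef returns the mode itself for other Blueprints.
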(event `self.ReceiveBeginPlay`
  (bind _settingstemp_audiosettings (break `/Game/Blueprints/Structs/STR_Settings` (`/Game/Blueprints/BP_GameInstance.settingsTemp` (`self.BP_GameInstance`))))
  (`|ExecutionSequence`
    (:`then_0`
      (bind _paddleref (message `/Game/Blueprints/Interfaces/BI_GetPaddle.GetPaddleRef` (`GameplayStatics.GetPlayerPawn` 0)))
      (bind _output_get (set `self.BP_Paddle` _paddleref))
      (bind _ballreference (`/Game/Blueprints/BP_Paddle.SpawnNewBall` _output_get))
      (set `self.BP_Ball` _ballreference))
    (:`then_1`
      (bind _gameinstanceref (message `/Game/Blueprints/Interfaces/BI_GetGameInstance.GetGameInstanceRef` (`GameplayStatics.GetGameInstance`)))
      (bind _output_get_2 (set `self.BP_GameInstance` _gameinstanceref))
      (`/Game/Blueprints/BP_GameInstance.LoadSavedData` _output_get_2)
      (for _array_element _settingstemp_audiosettings
        (`/Game/Blueprints/BP_GameInstance.ApplySoundSetting` (`self.BP_GameInstance`) _array_element)))))

(fn `GetGameModeRef`
  (returns (gmRef :type "/Game/Blueprints/BP_GameMode Object Reference") (menuGmRef :type "/Game/Blueprints/BP_GameMode_Menu Object Reference"))
  (return null self))

(fn `UserConstructionScript`)