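; Game mode for a paddle, ball and brick game that tracks lives, score, level progression and game end.
; On BeginPlay it caches HUD and paddle references via interface messages, spawns a ball and, outside the main menu, loads the save.
; Losing a life respawns the ball and resets bricks, or triggers game over.
; Cleared levels flag a wait for the next streamed level; game end saves the score and shows the game-over screen.
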(event `self.ReceiveBeginPlay`
  (`|ExecutionSequence`
    (:`then_0`
      (bind _hudref (message `/Game/Blueprints/Interfaces/BI_GetHUD.GetHudRef` (`PlayerController.GetHUD` (`GameplayStatics.GetPlayerController` 0))))
      (set `self.BP_HUD` _hudref))
    (:`then_1`
      (bind _paddleref (message `/Game/Blueprints/Interfaces/BI_GetPaddle.GetPaddleRef` (`GameplayStatics.GetPlayerPawn` 0)))
      (bind _output_get (set `self.BP_Paddle` _paddleref))
      (bind _ballreference (`/Game/Blueprints/BP_Paddle.SpawnNewBall` _output_get))
      (set `self.BP_Ball` _ballreference))
    (:`then_2`
      (bind _returnvalue (`GameplayStatics.GetCurrentLevelName` true))
      (if (`KismetStringLibrary.NotEqual_StrStr` _returnvalue "LevelMM")
        (bind _gameinstanceref (message `/Game/Blueprints/Interfaces/BI_GetGameInstance.GetGameInstanceRef` (`GameplayStatics.GetGameInstance`)))
        (bind _output_get_2 (set `self.BP_GameInstance` _gameinstanceref))
        (`/Game/Blueprints/BP_GameInstance.LoadSaveGame` _output_get_2)))))

(event `LoadLevelInd`
  (params (index :type Integer))
  (`GameplayStatics.LoadStreamLevelBySoftObjectPtr` (`|GetArrayItem` (`self.levels`) index) true)
  (set `self.waitingForNewLevel` false))

(fn `GetGameModeRef`
  (returns (gameModeRef :type "/Game/Blueprints/BP_GameMode Object Reference"))
  (return self))

(fn `IncrementScore`
  (params (scoreToAdd :type Integer))
  (bind _output_get (set `self.score` (+ scoreToAdd (`self.score`))))
  (`/Game/UI/WBP_HUD.UpdateDisplayedScore` (`/Game/UI/BP_HUD.WBP_HUD` (`self.BP_HUD`)) _output_get))

(fn `LoseLife`
  (params (oldBallReference :type "Actor Object Reference"))
  (`self.K2_DestroyActor` oldBallReference)
  (`/Engine/EditorBlueprintResources/StandardMacros.DecrementInt` (`self.nrLives`)
    (:`  `
      (`/Game/UI/WBP_LivesIndicator.RemoveLifeIcon` (`/Game/UI/WBP_HUD.WBP_LivesIndicator` (`/Game/UI/BP_HUD.WBP_HUD` (`self.BP_HUD`))))
      (if (> (`self.nrLives`) 0)
        (bind _ballreference (`/Game/Blueprints/BP_Paddle.SpawnNewBall` (`self.BP_Paddle`)))
        (set `self.BP_Ball` _ballreference)
        (`/Game/Blueprints/Actors/BP_GridForBricks.ResetBricks` (`self.BP_GridForBricks`))
        (else
          (`self.OnGameOver`))))))

(fn `OnGameCompleted`
  (`/Game/Blueprints/BP_GameInstance.CreateSaveGame` (`self.BP_GameInstance`) (`self.score`))
  (set `self.gameBeaten` true)
  (`GameplayStatics.SetGamePaused` true)
  (`/Game/UI/BP_HUD.DisplayUiWidget` (`self.BP_HUD`) (`/Game/UI/BP_HUD.WBP_GameOverScreen` (`self.BP_HUD`)) (`/Game/UI/WBP_MainMenuButton.Button_70` (`/Game/UI/WBP_GameOverScreen.WBP_MMBtn_Retry` (`/Game/UI/BP_HUD.WBP_GameOverScreen` (`self.BP_HUD`))))))

(fn `OnGameOver`
  (locals (NewLocalVar_0 :type "/Game/Blueprints/BP_SaveGame Object Reference"))
  (`/Game/Blueprints/BP_GameInstance.CreateSaveGame` (`self.BP_GameInstance`) (`self.score`))
  (`/Game/UI/BP_HUD.DisplayUiWidget` (`self.BP_HUD`) (`/Game/UI/BP_HUD.WBP_GameOverScreen` (`self.BP_HUD`)) (`/Game/UI/WBP_MainMenuButton.Button_70` (`/Game/UI/WBP_GameOverScreen.WBP_MMBtn_Retry` (`/Game/UI/BP_HUD.WBP_GameOverScreen` (`self.BP_HUD`))))))

(fn `OnLevelCleared`
  (if (== (`self.currentLevelIndex`) (`KismetArrayLibrary.Array_LastIndex` (`self.levels`)))
    (`self.OnGameCompleted`)
    (else
      (set `self.waitingForNewLevel` true))))

(fn `ReturnToMainMenu`
  (`GameplayStatics.OpenLevelBySoftObjectPtr` "/Game/Levels/LevelMM.LevelMM"))

(fn `StartNewGame`
  (`GameplayStatics.OpenLevelBySoftObjectPtr` "/Game/Levels/Level1.Level1"))

(fn `UserConstructionScript`)