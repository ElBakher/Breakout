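; BP_SaveGame is the save game object that persists top scores and audio settings in one slot.
; Separate resave functions each update one field and write the whole object to the slot, with a debug print after saving settings.
; The load function returns both fields from the loaded copy without copying them into itself, so a resave writes this instance's current value for the other field.
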(fn `LoadSaveGameFromSlot`
  (returns (topScoresSaved :type "Array of Integer") (settingsSaved :type "/Game/Blueprints/Structs/STR_Settings Structure"))
  (bind _returnvalue (`GameplayStatics.LoadGameFromSlot` (`self.slotName`)))
  (bind _asbp_save_game (cast `/Game/Blueprints/BP_SaveGame` _returnvalue))
  (return (`/Game/Blueprints/BP_SaveGame.topScoresSaved` _asbp_save_game) (`/Game/Blueprints/BP_SaveGame.audioSettingsSaved` _asbp_save_game)))

(fn `ResaveSettings`
  (params (newSettings :type "/Game/Blueprints/Structs/STR_Settings Structure"))
  (set `self.audioSettingsSaved` newSettings)
  (`GameplayStatics.SaveGameToSlot` self (`self.slotName`))
  (`KismetSystemLibrary.PrintString` null "settings saved"))

(fn `ResaveTopScores`
  (params (newTopScores :type "Array of Integer"))
  (set `self.topScoresSaved` newTopScores)
  (`GameplayStatics.SaveGameToSlot` self (`self.slotName`)))