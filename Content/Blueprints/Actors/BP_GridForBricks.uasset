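; Grid actor that lays out rows and columns of brick slots and fills them with BP_BrickBase actors at BeginPlay.
; The construction script derives spacing from the brick mesh bounds plus gaps, centering columns horizontally and stepping rows along negative local X.
; Each slot is a collisionless, semitransparent static mesh hidden in game, serving as an editor preview.
; At runtime, every child component of the root supplies a brick's spawn transform.
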(event `self.ReceiveBeginPlay`
  (`self.FillSlotsWithBricks`))

(fn `CalculateHorizOffset`
  (returns (ReturnValue :type "Float (double-precision)"))
  (return (* (- (* (`self.nrColumns`) 0.5) 0.5) (`self.horizSpacePerBrick`))))

(fn `FillSlotsWithBricks`
  (for _array_element (`SceneComponent.GetChildrenComponents` (`self.DefaultSceneRoot`) false)
    (`|SpawnActorFromClass` "/Game/Blueprints/Actors/Bricks/BP_BrickBase.BP_BrickBase_C" (`SceneComponent.K2_GetComponentToWorld` _array_element) "Undefined" "OverrideRootScale" null null)))

(fn `SetUpSlotMesh`
  (params (slotMesh :type "StaticMeshComponent Object Reference"))
  (`StaticMeshComponent.SetStaticMesh` slotMesh (`self.brickMesh`))
  (`PrimitiveComponent.SetCollisionEnabled` slotMesh "NoCollision")
  (`SceneComponent.SetHiddenInGame` slotMesh true false)
  (`PrimitiveComponent.CreateDynamicMaterialInstance` slotMesh 0 "/Game/Materials/M_Basic_Semitransparent.M_Basic_Semitransparent" "None"))

(fn `UserConstructionScript`
  (locals (createdSlot :type "StaticMeshComponent Object Reference") (currentVertOffset :type "Float (double-precision)" :default 0.0))
  (bind _returnvalue (`StaticMesh.GetBoundingBox` (`self.brickMesh`)))
  (`|ExecutionSequence`
    (:`then_0`
      (set `self.horizSpacePerBrick` (+ (- (.y (`.Max` (break `Box` _returnvalue))) (.y (break `Box` _returnvalue))) (`KismetMathLibrary.Conv_IntToDouble` (`self.horizGapSize`))))
      (set `self.vertSpacePerBrick` (+ (- (.x (`.Max` (break `Box` _returnvalue))) (.x (break `Box` _returnvalue))) (`KismetMathLibrary.Conv_IntToDouble` (`self.vertGapSize`))))
      (bind _output_get (set `self.horizOffset` (`self.CalculateHorizOffset`)))
      (`KismetSystemLibrary.PrintString` (`KismetStringLibrary.Conv_DoubleToString` _output_get)))
    (:`then_1`
      (for _index (range (`self.nrRows`))
        (set `local.currentVertOffset` (* (* _index (`self.vertSpacePerBrick`)) -1.0))
        (for _index_2 (range (`self.nrColumns`))
          (bind _returnvalue_2 (`AddComponent|NODE_AddStaticMeshComponent-0` :`bManualAttachment` true :`RelativeTransform` (`KismetMathLibrary.MakeTransform` (`KismetMathLibrary.MakeVector` (`local.currentVertOffset`) (- (* _index_2 (`self.horizSpacePerBrick`)) (`self.horizOffset`))) (struct) (1.0 1.0 1.0))))
          (bind _output_get_2 (set `local.createdSlot` _returnvalue_2))
          (`SceneComponent.K2_AttachToComponent` _output_get_2 (`self.DefaultSceneRoot`) "None" "KeepRelative" "KeepRelative" "KeepRelative" true)
          (`self.SetUpSlotMesh` (`local.createdSlot`)))))))