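; BP_Ball is a ball actor that bounces around at a constant DefaultSpeed, driven by a ProjectileMovement component.
; It holds still on BeginPlay until StartMoving launches it in a random direction within a 45-degree half-angle cone around world +X.
; AdjustReflectedVelocity bends its heading by adding a supplied vector to the normalized velocity, then rescales to DefaultSpeed.
; GetBallRef returns the actor itself.
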(event `self.ReceiveBeginPlay`
  (set `MovementComponent.Velocity` (0.0 0.0 0.0) (`self.ProjectileMovement`)))

(fn `AdjustReflectedVelocity`
  (params (vectorToAdd :type "Vector Structure"))
  (set `MovementComponent.Velocity` (* (`KismetMathLibrary.Normal` (+ vectorToAdd (`KismetMathLibrary.Normal` (`MovementComponent.Velocity` (`self.ProjectileMovement`)) 0.01)) 0.01) (`self.defaultSpeed`)) (`self.ProjectileMovement`)))

(fn `GetBallRef`
  (returns (ballRef :type "/Game/Blueprints/Actors/BP_Ball Object Reference"))
  (return self))

(fn `StartMoving`
  (set `MovementComponent.Velocity` (* (`KismetMathLibrary.RandomUnitVectorInConeInDegrees` (1.0 0.0 0.0) 45.0) (`self.defaultSpeed`)) (`self.ProjectileMovement`)))

(fn `UserConstructionScript`)