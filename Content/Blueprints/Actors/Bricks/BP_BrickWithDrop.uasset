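; BP_BrickWithDrop is a brick actor that leaves a drop behind when it is destroyed.
; On BeginPlay it runs the parent logic and binds SpawnDrop to its own OnDestroyed event.
; SpawnDrop spawns the Drop class at the static mesh's world location, but skips it while BPGridForBricks flags ResettingBricks, so grid resets yield no drops.
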(event `self.ReceiveBeginPlay`
  (`parent.ReceiveBeginPlay`)
  (add `Actor.OnDestroyed` (delegate `SpawnDrop`)))

(event `SpawnDrop`
  (params (DestroyedActor :type "Actor Object Reference"))
  (if (not (`/Game/Blueprints/Actors/BP_GridForBricks.resettingBricks` (`self.BP_GridForBricks`)))
    (`|SpawnActorFromClass` (`self.drop`) (`KismetMathLibrary.MakeTransform` (`SceneComponent.K2_GetComponentLocation` (`self.StaticMesh`))) "Undefined" "OverrideRootScale" null null)))

(fn `UserConstructionScript`
  (`parent.UserConstructionScript`))