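; BP_BrickBase is the base brick actor for a ball-and-brick game, losing HP when hit by an actor implementing BI_GetBall.
; At zero HP it spawns particles, adds its score through the game mode, notifies BPGridForBricks and destroys itself.
; During a grid reset, a hit removes it without sound, particles or score.
; Construction applies a dynamic material, tinting M_Basic, while the optional widget icon waits until BeginPlay.
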(event `self.ReceiveBeginPlay`
  (bind _gamemoderef (message `/Game/Blueprints/Interfaces/BI_GetGameMode.GetGameModeRef` (`GameplayStatics.GetGameMode`)))
  (set `self.BP_GameMode` _gamemoderef)
  (`self.SetUpIcon`) ; has to be called here - construction script is apparently too early
)

(event `self.StaticMesh.OnComponentHit`
  (params (HitComponent :type "PrimitiveComponent Object Reference") (OtherActor :type "Actor Object Reference") (OtherComp :type "PrimitiveComponent Object Reference") (NormalImpulse :type "Vector Structure") (Hit :type "HitResult Structure (by ref)"))
  (`/Game/Blueprints/Libraries/MacroLibrary.DoesImplementInterface` OtherActor "/Game/Blueprints/Interfaces/BI_GetBall.BI_GetBall_C"
    (:`True`
      (`self.RegisterBallHit`))))

(fn `GetBrickRef`
  (returns (brickRef :type "/Game/Blueprints/Actors/Bricks/BP_BrickBase Object Reference"))
  (return self))

(fn `RegisterBallHit`
  (locals (brickLocation :type "Vector Structure" :default (0.0 0.0 0.0)))
  (set `local.brickLocation` (`SceneComponent.K2_GetComponentLocation` (`self.StaticMesh`)))
  (if (`/Game/Blueprints/Actors/BP_GridForBricks.resettingBricks` (`self.BP_GridForBricks`))
    (`/Game/Blueprints/Actors/BP_GridForBricks.OnBrickDestroyed` (`self.BP_GridForBricks`) self :!label _label)
    (`self.K2_DestroyActor`)
    (else
      (`GameplayStatics.PlaySoundAtLocation` (`self.hitSound`) (`local.brickLocation`) (struct) 1.0 1.0 0.0 null null null)
      (bind _result (`/Engine/EditorBlueprintResources/StandardMacros.DecrementInt` (`self.HP`))
        (:`  `
          (if (== _result 0)
            (`GameplayStatics.SpawnEmitterAtLocation` (`self.hitParticle`) (`local.brickLocation`))
            (`/Game/Blueprints/BP_GameMode.IncrementScore` (`self.BP_GameMode`) (`self.scoreValue`))
            (goto _label)))))))

(fn `SetUpIcon`
  (`self.brickIcon`
    (:`then`
      (bind _brickiconref (message `/Game/Blueprints/Interfaces/BI_GetBrickIcon.GetBrickIcon` (`WidgetComponent.GetUserWidgetObject` (`self.BrickIconWidget`))))
      (`/Game/UI/WBP_BrickIcon.SetTextureAndVisibility` _brickiconref (`self.brickIcon`)))
    (:`else`)))

(fn `SetUpVisuals`
  (bind _returnvalue (`PrimitiveComponent.CreateDynamicMaterialInstance` (`self.StaticMesh`) 0 (`self.sourceMaterial`) "None"))
  (if (== (`self.sourceMaterial`) "/Game/Materials/M_Basic.M_Basic")
    (`MaterialInstanceDynamic.SetVectorParameterValue` _returnvalue "Color" (`self.meshColor`))
    (`self.brickIcon`
      (:`then`)
      (:`else`))))

(fn `UserConstructionScript`
  (`self.SetUpVisuals`))