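; BP_BrickShooting is a brick actor with a cannon that fires bombs at a regular interval.
; A looping timer started on BeginPlay calls Shoot, which spawns a BP_DroppedBomb at the bomb spawn point and plays a launch sound there.
; Each shot also triggers the OnShoot event, where a timeline drives the cannon's relative Y location for a blowback animation.
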(event `self.ReceiveBeginPlay`
  (`parent.ReceiveBeginPlay`)
  (`KismetSystemLibrary.K2_SetTimer` null "Shoot" (`self.delayBetweenShots`) true))

(event `OnShoot`
  (bind (_direction _cannonoffset) (`Timeline|CannonBlowback` :!via `PlayFromStart`)
    (:`Update`
      (`SceneComponent.K2_SetRelativeLocation` (`self.Cannon`) (`KismetMathLibrary.MakeVector` 0.0 _cannonoffset) false false))))

(fn `Shoot`
  (bind _bombspawnpoint (`self.BombSpawnPoint`))
  (`self.OnShoot`)
  (`|SpawnActorFromClass` "/Game/Blueprints/Actors/Drops/BP_DroppedBomb.BP_DroppedBomb_C" (`SceneComponent.K2_GetComponentToWorld` _bombspawnpoint) "AlwaysSpawn" "OverrideRootScale" null null)
  (`GameplayStatics.PlaySoundAtLocation` (`self.bombLaunchSound`) (`SceneComponent.K2_GetComponentLocation` _bombspawnpoint) (struct) 1.0 1.0 0.0 null null null))

(fn `UserConstructionScript`
  (`parent.UserConstructionScript`))