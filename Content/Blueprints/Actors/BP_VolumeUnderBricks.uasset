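; Trigger volume, named as sitting under the bricks, that starts the next level when the ball enters it while the game mode is waiting for a new level.
; BeginPlay caches the game mode reference through GetGameModeRefMessage.
; Overlaps from BI_GetBall actors increment the game mode's level index and load that level.
; A DoOnce wraps the load and resets immediately afterward.
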(event `self.ReceiveBeginPlay`
  (bind _gamemoderef (message `/Game/Blueprints/Interfaces/BI_GetGameMode.GetGameModeRef` (`GameplayStatics.GetGameMode`)))
  (set `self.BP_GameMode` _gamemoderef))

(event `self.BallAreaAllowingBricksSpawn.OnComponentBeginOverlap`
  (params (OverlappedComponent :type "PrimitiveComponent Object Reference") (OtherActor :type "Actor Object Reference") (OtherComp :type "PrimitiveComponent Object Reference") (OtherBodyIndex :type Integer) (bFromSweep :type Boolean) (SweepResult :type "HitResult Structure (by ref)"))
  (if (`/Game/Blueprints/BP_GameMode.waitingForNewLevel` (`self.BP_GameMode`))
    (`/Game/Blueprints/Libraries/MacroLibrary.DoesImplementInterface` OtherActor "/Game/Blueprints/Interfaces/BI_GetBall.BI_GetBall_C"
      (:`True`
        (`/Engine/EditorBlueprintResources/StandardMacros.DoOnce` false :!label _label
          (:`Completed`
            (`/Engine/EditorBlueprintResources/StandardMacros.IncrementInt` (`/Game/Blueprints/BP_GameMode.currentLevelIndex` (`self.BP_GameMode`))
              (:`  `
                (`/Game/Blueprints/BP_GameMode.LoadLevelInd` (`self.BP_GameMode`) (`/Game/Blueprints/BP_GameMode.currentLevelIndex` (`self.BP_GameMode`)))
                (goto _label :!via `Reset`)))))))))

(fn `UserConstructionScript`)