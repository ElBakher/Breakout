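; BP_PlayArea is the bounded play area actor for a ball game, detecting lost balls and boundary impacts.
; It gets the game mode reference on BeginPlay.
; Overlaps with GameOverMesh call LoseLife on the game mode for BI_GetBall actors, while other actors tagged "destroy" are destroyed.
; Hits on PlayAreaBoundsMesh play a sound at the impact location.
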(event `self.ReceiveBeginPlay`
  (bind _gamemoderef (message `/Game/Blueprints/Interfaces/BI_GetGameMode.GetGameModeRef` (`GameplayStatics.GetGameMode`)))
  (set `self.BP_GameMode` _gamemoderef))

(event `self.GameOverMesh.OnComponentBeginOverlap`
  (params (OverlappedComponent :type "PrimitiveComponent Object Reference") (OtherActor :type "Actor Object Reference") (OtherComp :type "PrimitiveComponent Object Reference") (OtherBodyIndex :type Integer) (bFromSweep :type Boolean) (SweepResult :type "HitResult Structure (by ref)"))
  (`/Game/Blueprints/MacroLibrary.DoesImplementInterface` OtherActor "/Game/Blueprints/Interfaces/BI_GetBall.BI_GetBall_C"
    (:`True`
      (`/Game/Blueprints/BP_GameMode.LoseLife` (`self.BP_GameMode`) OtherActor))
    (:`False`
      (if (`self.ActorHasTag` OtherActor "destroy")
        (`self.K2_DestroyActor` OtherActor)))))

(event `self.PlayAreaBoundsMesh.OnComponentHit`
  (params (HitComponent :type "PrimitiveComponent Object Reference") (OtherActor :type "Actor Object Reference") (OtherComp :type "PrimitiveComponent Object Reference") (NormalImpulse :type "Vector Structure") (Hit :type "HitResult Structure (by ref)"))
  (`GameplayStatics.PlaySoundAtLocation` null (`.Location` (`GameplayStatics.BreakHitResult` Hit)) (struct) 1.0 1.0 0.0 null null null))

(fn `UserConstructionScript`)