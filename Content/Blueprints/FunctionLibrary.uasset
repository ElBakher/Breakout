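; Blueprint function library with a helper that closes a UI widget from an ordered array of widgets.
; CloseUiWidget collapses the given widget, then searches backward from its array position for the nearest earlier non-collapsed widget and makes it visible, acting like a menu stack.
; When none is found, it switches the first player controller to game-only input and hides the mouse cursor.
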(fn `CloseUiWidget`
  (params (widgetToClose :type "UserWidget Object Reference") (uiWidgets :type "Array of UserWidget Object Reference"))
  (locals (lastInd :type Integer :default 0) (uiWidgetInd_i :type "UserWidget Object Reference"))
  (`Widget.SetVisibility` (`local.widgetToClose`) "Collapsed")
  (bind _output_get (set `local.lastInd` (- (`KismetArrayLibrary.Array_Find` (`local.uiWidgets`) (`local.widgetToClose`)) 1)))
  (for _index (range (+ _output_get 1))
    (bind _output_get_2 (set `local.uiWidgetInd_i` (`|GetArrayItem` (`local.uiWidgets`) (- (`local.lastInd`) _index))))
    (if (`|EnumInequality` (`Widget.GetVisibility` _output_get_2) "Collapsed")
      (`Widget.SetVisibility` (`local.uiWidgetInd_i`) "Visible")
      (return)))
  (`WidgetBlueprintLibrary.SetInputMode_GameOnly` (`GameplayStatics.GetPlayerController` null))
  (set `PlayerController.bShowMouseCursor` false (`GameplayStatics.GetPlayerController` null)))