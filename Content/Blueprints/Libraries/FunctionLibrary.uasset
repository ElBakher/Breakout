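; Blueprint function library that opens and closes layered UI widgets, using the caller's array order as the stack.
; DisplayUiWidget sets visible widgets earlier in the array to SelfHitTestInvisible, shows the target, and enables UI-only input with cursor if the cursor is hidden.
; CloseUiWidget collapses the target and restores the nearest preceding non-collapsed widget to Visible, or returns player 0 to game-only input without a cursor.
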(fn `CloseUiWidget`
  (params (widgetToClose :type "UserWidget Object Reference") (uiWidgets :type "Array of UserWidget Object Reference"))
  (locals (lastInd :type Integer :default 0) (uiWidgetInd_i :type "UserWidget Object Reference"))
  (bind _returnvalue (`GameplayStatics.GetPlayerController` null))
  (`Widget.SetVisibility` (`local.widgetToClose`) "Collapsed")
  (bind _output_get (set `local.lastInd` (- (`KismetArrayLibrary.Array_Find` (`local.uiWidgets`) (`local.widgetToClose`)) 1)))
  (for _index (range (+ _output_get 1))
    (bind _output_get_2 (set `local.uiWidgetInd_i` (`|GetArrayItem` (`local.uiWidgets`) (- (`local.lastInd`) _index))))
    (if (`|EnumInequality` (`Widget.GetVisibility` _output_get_2) "Collapsed")
      (`Widget.SetVisibility` (`local.uiWidgetInd_i`) "Visible")
      (return)))
  (`WidgetBlueprintLibrary.SetInputMode_GameOnly` _returnvalue)
  (set `PlayerController.bShowMouseCursor` false _returnvalue))

(fn `DisplayUiWidget`
  (params (widgetToDisplay :type "UserWidget Object Reference") (uiWidgets :type "Array of UserWidget Object Reference"))
  (locals (uiWidgetInd_i :type "UserWidget Object Reference"))
  (bind _returnvalue (`GameplayStatics.GetPlayerController` null))
  (for _index (range (`KismetArrayLibrary.Array_Find` uiWidgets (`local.widgetToDisplay`)))
    (bind _output_get (set `local.uiWidgetInd_i` (`|GetArrayItem` (`local.uiWidgets`) _index)))
    (if (`|EnumEquality` (`Widget.GetVisibility` _output_get) "Visible")
      (`Widget.SetVisibility` (`local.uiWidgetInd_i`) "SelfHitTestInvisible")))
  (`Widget.SetVisibility` (`local.widgetToDisplay`) "Visible")
  (if (not (`PlayerController.bShowMouseCursor` (`GameplayStatics.GetPlayerController` null)))
    (`WidgetBlueprintLibrary.SetInputMode_UIOnlyEx` _returnvalue null)
    (set `PlayerController.bShowMouseCursor` true _returnvalue)))